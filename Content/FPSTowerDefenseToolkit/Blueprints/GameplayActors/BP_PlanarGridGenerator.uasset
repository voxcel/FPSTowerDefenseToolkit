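; BP_PlanarGridGenerator is a placeable flat, rotatable grid that defines tower placement cells for tower defense levels.
; The construction script scales the floor mesh from cell counts and BP_GridManager's cell size, then builds cell centers along the actor's axes.
; Instanced meshes preview cells in the editor and clear at BeginPlay unless display is enabled.
; Via BPI_GridLink, it projects trace hits onto those axes, returning cell index, generator index and position.
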(event `self.ReceiveBeginPlay`
  ;[1 0 0 0.5] Clear all the grid cell instances based on 'DisplayGridCells?' parameter
  (if (not (`self.DisplayGridCells?`))
    (`InstancedStaticMeshComponent.ClearInstances` (`self.InstancedGridCell`))))

(fn `CreateGridArray`
  (params (GridCellSize :type "Float (double-precision)"))
  (returns (Output_GridArray :type "Array of Vector Structure"))
  (locals (Local_GridCellSize :type "Float (double-precision)"))
  (bind _local_gridcellsize (`local.Local_GridCellSize`))
  (bind _returnvalue (/ (`local.Local_GridCellSize`) 2.0))
  (bind _returnvalue_2 (/ _local_gridcellsize 2.0))
  ;[0 1 1 0.5] Upgraded to add support for 360 rotation of Grid Generators; Calculates Grid Details based on the underlying Grid mesh and grid size
  (set `local.Local_GridCellSize` GridCellSize)
  (set `self.StartingVector` (+ (- (- (`KismetSystemLibrary.GetComponentBounds` (`self.GridMesh`)) (* (`self.GetActorRightVector`) (* _returnvalue (`KismetMathLibrary.Conv_IntToDouble` (`self.GridCountY`))))) (* (`self.GetActorForwardVector`) (* _returnvalue (`KismetMathLibrary.Conv_IntToDouble` (`self.GridCountX`))))) (* (`self.GetActorUpVector`) 50.0)))
  (for _index (range (`self.GridCountX`))
    (for _index_2 (range (`self.GridCountY`))
      (`KismetArrayLibrary.Array_Add` (`self.GridArray`) (+ (`self.StartingVector`) (+ (* (`self.GetActorRightVector`) (+ (* _index_2 _local_gridcellsize) _returnvalue_2)) (* (`self.GetActorForwardVector`) (+ (* _index _local_gridcellsize) _returnvalue_2)))))))
  (return (`self.GridArray`)))

(fn `RetrieveTraceHitGridData`
  (params (TraceHitLocation :type "Vector Structure"))
  (returns (GridCellIndex :type Integer) (GridGeneratorIndex :type Integer) (GridVector :type "Vector Structure"))
  (locals (Local_GridCellIndex :type Integer) (Local_GridCellSize :type "Float (double-precision)" :default 0.0))
  (bind _local_gridcellsize (`local.Local_GridCellSize`))
  (bind _startingvector (`self.StartingVector`))
  (bind _gridmanagerref (`/Game/FPSTowerDefenseToolkit/Blueprints/FunctionLibraries/BPFL_GetterFunctions.GetGridManager` self))
  ;[0 1 0.4 0.5] 'BPI_GridLink' interface function used to retrieve grid data of the implementing actor
  (`/Engine/EditorBlueprintResources/StandardMacros.IsValid` _gridmanagerref
    (:`Is Valid`
      (set `local.Local_GridCellSize` (`/Game/FPSTowerDefenseToolkit/Blueprints/GameplayActors/BP_GridManager.RetrieveGridCellSize` _gridmanagerref)))
    (:`Is Not Valid`
      (bind _outactors (`GameplayStatics.GetAllActorsOfClass` "/Game/FPSTowerDefenseToolkit/Blueprints/GameplayActors/BP_GridManager.BP_GridManager_C"))
      (set `local.Local_GridCellSize` (`/Game/FPSTowerDefenseToolkit/Blueprints/GameplayActors/BP_GridManager.RetrieveGridCellSize` (`KismetArrayLibrary.Array_Get` _outactors)))))
  (set `local.Local_GridCellIndex` (+ (* (`self.GridCountY`) (`KismetMathLibrary.FFloor` (/ (`KismetMathLibrary.VSize` (`KismetMathLibrary.ProjectVectorOnToVector` (- TraceHitLocation _startingvector) (`self.GetActorForwardVector`))) _local_gridcellsize))) (`KismetMathLibrary.FFloor` (/ (`KismetMathLibrary.VSize` (`KismetMathLibrary.ProjectVectorOnToVector` (- TraceHitLocation _startingvector) (`self.GetActorRightVector`))) _local_gridcellsize))))
  (return (`local.Local_GridCellIndex`) (`self.GeneratorIndex`) (`KismetArrayLibrary.Array_Get` (`self.GridArray`) (`local.Local_GridCellIndex`))))

(fn `SetGeneratorIndex`
  (params (Index :type Integer))
  ;[0 1 1 0.5] Sets a unique grid generator index for the actor
  (set `self.GeneratorIndex` Index)
  (return))

(fn `UserConstructionScript`
  (locals (Local_GridCellSize :type "Float (double-precision)" :default 0.0))
  (bind _local_gridcellsize (`local.Local_GridCellSize`))
  (bind (_min _max) (`StaticMeshComponent.GetLocalBounds` (`self.GridMesh`)))
  ;[0 1 1 0.5] Scales the Grid Floor based on the user defined grid counts in X & Y directions; Create Grid Instances for visualizing Tower Placement locations during level design
  (`parent.UserConstructionScript`)
  (bind _outactors (`GameplayStatics.GetAllActorsOfClass` "/Game/FPSTowerDefenseToolkit/Blueprints/GameplayActors/BP_GridManager.BP_GridManager_C"))
  (set `local.Local_GridCellSize` (`/Game/FPSTowerDefenseToolkit/Blueprints/GameplayActors/BP_GridManager.GridCellSize` (`KismetArrayLibrary.Array_Get` _outactors)))
  (set `self.DefaultGridMeshBounds` (- _max _min))
  (`SceneComponent.SetWorldScale3D` (`self.GridMesh`) (`KismetMathLibrary.MakeVector` (/ (* (`KismetMathLibrary.Conv_IntToDouble` (`self.GridCountX`)) _local_gridcellsize) (.x (`self.DefaultGridMeshBounds`))) (/ (* (`KismetMathLibrary.Conv_IntToDouble` (`self.GridCountY`)) _local_gridcellsize) (.y (`self.DefaultGridMeshBounds`))) 1.0))
  (bind _output_gridarray (`self.CreateGridArray` (`local.Local_GridCellSize`)))
  (for _array_element _output_gridarray
    (`InstancedStaticMeshComponent.AddInstanceWorldSpace` (`self.InstancedGridCell`) (`KismetMathLibrary.MakeTransform` (`KismetMathLibrary.MakeVector` (.x _array_element) (.y _array_element) (+ (.z _array_element) 1.0)) (`self.K2_GetActorRotation`)))))
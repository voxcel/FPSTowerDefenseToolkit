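; Tower defense spawn point that spawns timed creep batches inside a box volume, facing the Power Core, and reports to the Wave Manager.
; Batch events are per class and live here so simultaneous groups from different points don't conflict.
; Spawn transforms are random, optionally cached at initialization.
; It also draws a spline-mesh navmesh path to the Core and shows upcoming creep counts (except threat-based waves) on a player-facing 3D widget.
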(event `self.ReceiveTick`
  (params (DeltaSeconds :type "Float (single-precision)"))
  (bind _returnvalue (`GameplayStatics.GetPlayerCharacter` 0))
  ;[0 1 1 0.5] Keep the Wave Data Widget facing the player at all times
  (`/Engine/EditorBlueprintResources/StandardMacros.IsValid` _returnvalue
    (:`Is Valid`
      (`SceneComponent.K2_SetRelativeRotation` (`self.WaveSpawnDataDisplayComponent`) (`KismetMathLibrary.MakeRotator` 90.0 0.0 (- (.yaw (`KismetMathLibrary.FindLookAtRotation` (`SceneComponent.K2_GetComponentLocation` (`self.WaveSpawnDataDisplayComponent`)) (`self.K2_GetActorLocation` _returnvalue))) 90.0)) false false))))

(event `CreateNavPath`
  (bind _pathspline (`self.PathSpline`))
  (bind _pathspline_2 (`self.PathSpline`))
  (bind _splineheight (`self.SplineHeight`))
  (bind _splinemesharray (`self.SplineMeshArray`))
  (bind _powercore (`/Game/FPSTowerDefenseToolkit/Blueprints/FunctionLibraries/BPFL_GetterFunctions.GetPowerCore` self))
  ;[0 1 1 0.5] Create Navigation Path for the Enemy Bots
  (`KismetSystemLibrary.Delay` 0.1) ; Waits for nav rebuild to finish execution
  (`/Engine/EditorBlueprintResources/StandardMacros.IsValid` _powercore
    (:`Is Valid`
      (for _array_element _splinemesharray
        (`ActorComponent.K2_DestroyComponent` _array_element) ; Destroy existing spline mesh components before creating a new one
      )
      (`KismetArrayLibrary.Array_Clear` _splinemesharray)
      (bind _returnvalue (`NavigationSystem.FindPathToLocationSynchronously` (`NavigationSystem.ProjectPointToNavigation` (`self.K2_GetActorLocation`)) (`NavigationSystem.ProjectPointToNavigation` (`self.K2_GetActorLocation` _powercore) null null (0.0 0.0 0.0)))) ; Get path points from the spawn point to the Power Core
      (set `self.PathArray` (`NavigationPath.PathPoints` _returnvalue))
      (if (> (`KismetArrayLibrary.Array_Length` (`self.PathArray`)) 1)
        (`SplineComponent.SetSplinePoints` _pathspline (`self.PathArray`) "World" true)
        (for _index (range (+ (- (`SplineComponent.GetNumberOfSplinePoints` _pathspline) 2) 1))
          (bind _returnvalue_2 (`AddComponent|SplineMeshComponent_0`))
          (bind _output_get (set `self.SplineMesh` _returnvalue_2))
          (`StaticMeshComponent.SetStaticMesh` _output_get "/Game/FPSTowerDefenseToolkit/Meshes/SM_NavPathSpline.SM_NavPathSpline")
          (`PrimitiveComponent.CreateDynamicMaterialInstance` _output_get 0 "/Game/FPSTowerDefenseToolkit/Materials/M_Emissive.M_Emissive")
          (bind (_location _tangent) (`SplineComponent.GetLocationAndTangentAtSplinePoint` _pathspline_2 _index "Local"))
          (bind (_location_2 _tangent_2) (`SplineComponent.GetLocationAndTangentAtSplinePoint` _pathspline_2 (+ _index 1) "Local"))
          (`SplineMeshComponent.SetStartAndEnd` (`self.SplineMesh`) (`KismetMathLibrary.MakeVector` (.x _location) (.y _location) (+ (.z _location) _splineheight)) (`KismetMathLibrary.MakeVector` (.x _tangent) (.y _tangent) (+ (.z _tangent) _splineheight)) (`KismetMathLibrary.MakeVector` (.x _location_2) (.y _location_2) (+ (.z _location_2) _splineheight)) (`KismetMathLibrary.MakeVector` (.x _tangent_2) (.y _tangent_2) (+ (.z _tangent_2) _splineheight)) true)
          (`KismetArrayLibrary.Array_Add` (`self.SplineMeshArray`) (`self.SplineMesh`)))))))

(event `SpawnCreepBatch_CoreBomberClass`
  (params (StartDelay :type "Float (double-precision)") (NumberOfCreeps :type Integer) (SpawnInterval :type "Float (double-precision)") (CreepClass :type "/Game/FPSTowerDefenseToolkit/Blueprints/EnemyAI/BP_EnemyAI_Parent Class Reference") (CycleMultiplier :type Integer))
  ;[0 1 1 0.5] Spawns batches of creeps based on the specified input parameters [Moved here from the Wave Manager to prevent a bug that arises from event access conflict when multiple groups of the same creep class are spawned from multiple enemy spawn points in the same time frame. Now with the spawn logic moved to the spawn points, each spawn point has it's own set of events that can be called upon without interfering with the other spawn points.
  (`KismetSystemLibrary.Delay` StartDelay)
  (`self.ForLoopWithDelay` 1 NumberOfCreeps SpawnInterval
    (:`LoopBody`
      (`self.SpawnCreep` CreepClass CycleMultiplier))
    (:`Completed`
      (`/Game/FPSTowerDefenseToolkit/Blueprints/GameplayActors/BP_WaveManager.DecrementNumberOfActiveSpawnGroups` (`/Game/FPSTowerDefenseToolkit/Blueprints/FunctionLibraries/BPFL_GetterFunctions.GetWaveManager` self)))))

(event `SpawnCreepBatch_MeleeClass`
  (params (StartDelay :type "Float (double-precision)") (NumberOfCreeps :type Integer) (SpawnInterval :type "Float (double-precision)") (CreepClass :type "/Game/FPSTowerDefenseToolkit/Blueprints/EnemyAI/BP_EnemyAI_Parent Class Reference") (CycleMultiplier :type Integer))
  ;[0 1 1 0.5] Spawns batches of creeps based on the specified input parameters [Moved here from the Wave Manager to prevent a bug that arises from event access conflict when multiple groups of the same creep class are spawned from multiple enemy spawn points in the same time frame. Now with the spawn logic moved to the spawn points, each spawn point has it's own set of events that can be called upon without interfering with the other spawn points.
  (`KismetSystemLibrary.Delay` StartDelay)
  (`self.ForLoopWithDelay` 1 NumberOfCreeps SpawnInterval
    (:`LoopBody`
      (`self.SpawnCreep` CreepClass CycleMultiplier))
    (:`Completed`
      (`/Game/FPSTowerDefenseToolkit/Blueprints/GameplayActors/BP_WaveManager.DecrementNumberOfActiveSpawnGroups` (`/Game/FPSTowerDefenseToolkit/Blueprints/FunctionLibraries/BPFL_GetterFunctions.GetWaveManager` self)))))

(event `SpawnCreepBatch_RangedClass`
  (params (StartDelay :type "Float (double-precision)") (NumberOfCreeps :type Integer) (SpawnInterval :type "Float (double-precision)") (CreepClass :type "/Game/FPSTowerDefenseToolkit/Blueprints/EnemyAI/BP_EnemyAI_Parent Class Reference") (CycleMultiplier :type Integer))
  ;[0 1 1 0.5] Spawns batches of creeps based on the specified input parameters [Moved here from the Wave Manager to prevent a bug that arises from event access conflict when multiple groups of the same creep class are spawned from multiple enemy spawn points in the same time frame. Now with the spawn logic moved to the spawn points, each spawn point has it's own set of events that can be called upon without interfering with the other spawn points.
  (`KismetSystemLibrary.Delay` StartDelay)
  (`self.ForLoopWithDelay` 1 NumberOfCreeps SpawnInterval
    (:`LoopBody`
      (`self.SpawnCreep` CreepClass CycleMultiplier))
    (:`Completed`
      (`/Game/FPSTowerDefenseToolkit/Blueprints/GameplayActors/BP_WaveManager.DecrementNumberOfActiveSpawnGroups` (`/Game/FPSTowerDefenseToolkit/Blueprints/FunctionLibraries/BPFL_GetterFunctions.GetWaveManager` self)))))

(fn `CreateCachedSpawnTransforms`
  ;[0 1 1 0.5] Creates a set of spawn transforms at level start; Improves runtime performance as the spawn transforms can be retrieved randomly from the array instead of creating them at each & every spawn event
  (for _ (range 1 (+ (`self.NumberOfCachedSpawnTransforms`) 1))
    (`KismetArrayLibrary.Array_Add` (`self.CachedBotSpawnTransforms`) (`self.CreateRandomSpawnTransform`)))
  (return))

(fn `CreateRandomSpawnTransform`
  (returns (SpawnTransform :type "Transform Structure"))
  (bind (_returnvalue_x _returnvalue_y) (`KismetMathLibrary.BreakVector` (`BoxComponent.GetScaledBoxExtent` (`self.SpawningVolume`))))
  ;[0 1 1 0.5] Creates a random spawn location within the spawning volume
  (return (`KismetMathLibrary.MakeTransform` (+ (`self.K2_GetActorLocation`) (`KismetMathLibrary.MakeVector` (`KismetMathLibrary.RandomFloatInRange` (* _returnvalue_x -1.0) _returnvalue_x) (`KismetMathLibrary.RandomFloatInRange` (* _returnvalue_y -1.0) _returnvalue_y) (`self.SpawnHeightOffset`))) (`KismetMathLibrary.FindLookAtRotation` (`self.K2_GetActorLocation`) (`self.K2_GetActorLocation` (`/Game/FPSTowerDefenseToolkit/Blueprints/FunctionLibraries/BPFL_GetterFunctions.GetPowerCore` self))))))

(fn `DisplayWaveSpawnInformation`
  (locals (Local_CreepSpawnCountData :type "Array of /Game/FPSTowerDefenseToolkit/Blueprints/Structs/Struct_CreepSpawnCounter Structure"))
  (bind _wavemanager (`/Game/FPSTowerDefenseToolkit/Blueprints/FunctionLibraries/BPFL_GetterFunctions.GetWaveManager` self))
  ;[0 1 1 0.5] Displays the spawn count data for every creep that is to be spawned from this spawn point in the upcoming wave [Ignored for threat based wave generation as the spawn points & creeps are spawned randomly]
  (switch `/Game/FPSTowerDefenseToolkit/Blueprints/Enums/EWaveGenerator` (`/Game/FPSTowerDefenseToolkit/Blueprints/GameplayActors/BP_WaveManager.RetrieveWaveGeneratorType` (`/Game/FPSTowerDefenseToolkit/Blueprints/FunctionLibraries/BPFL_GetterFunctions.GetWaveManager` self))
    (:`NewEnumerator0`
      (bind _creepspawncountdata (`/Game/FPSTowerDefenseToolkit/Blueprints/GameplayActors/BP_WaveManager.RetrieveUnitBasedCreepSpawnCountData` _wavemanager self))
      (set `local.Local_CreepSpawnCountData` _creepspawncountdata)
      (if (> (`KismetArrayLibrary.Array_Length` (`local.Local_CreepSpawnCountData`)) 0) :!label _label
        (for _array_element (`local.Local_CreepSpawnCountData`)
          (bind (_creepclass _spawncount) (break `/Game/FPSTowerDefenseToolkit/Blueprints/Structs/Struct_CreepSpawnCounter` _array_element))
          (bind _returnvalue (`|CreateWidget` (`self.StatsWidgetClassRef`) (`GameplayStatics.GetPlayerController` 0) (`KismetTextLibrary.Conv_StringToText` (`|GetEnumeratorNameAsString` (defaults `/Game/FPSTowerDefenseToolkit/Blueprints/GameplayActors/BP_EnemySpawnPoint` _creepclass))) _spawncount)) ; Create a stats widget to display the creep spawn count
          (bind _aswidget_wave_spawn_details (cast `/Game/FPSTowerDefenseToolkit/UI/Widgets/Widget_WaveSpawnDetails` (`WidgetComponent.GetUserWidgetObject` (`self.WaveSpawnDataDisplayComponent`))))
          (`/Game/FPSTowerDefenseToolkit/UI/Widgets/Widget_WaveSpawnDetails.AddNewStatsToWaveData` _aswidget_wave_spawn_details _returnvalue) ; Add the stats widget to the 3D Widget one by one
        )
        (`self.SetActorTickEnabled` true) ; Makes the 3D Widget rotate to face the player
        (`SceneComponent.SetVisibility` (`self.WaveSpawnDataDisplayComponent`) true false)
        (else
          (`SceneComponent.SetVisibility` (`self.WaveSpawnDataDisplayComponent`) false false :!label _label_2)
          (`self.SetActorTickEnabled` false))))
    (:`NewEnumerator1`
      (bind _creepspawncountdata_2 (`/Game/FPSTowerDefenseToolkit/Blueprints/GameplayActors/BP_WaveManager.RetrieveGroupBasedCreepSpawnCountData` _wavemanager self))
      (set `local.Local_CreepSpawnCountData` _creepspawncountdata_2)
      (goto _label))
    (:`NewEnumerator2`
      (goto _label_2))))

(fn `HideWaveSpawnInformation`
  ;[0 1 1 0.5] Hide the wave data 3D widget & reset it's content
  (`SceneComponent.SetVisibility` (`self.WaveSpawnDataDisplayComponent`) false false)
  (bind _aswidget_wave_spawn_details (cast `/Game/FPSTowerDefenseToolkit/UI/Widgets/Widget_WaveSpawnDetails` (`WidgetComponent.GetUserWidgetObject` (`self.WaveSpawnDataDisplayComponent`))))
  (`/Game/FPSTowerDefenseToolkit/UI/Widgets/Widget_WaveSpawnDetails.ResetWaveData` _aswidget_wave_spawn_details)
  (`self.SetActorTickEnabled` false))

(fn `InitializeEnemySpawnPoint`
  ;[0 1 1 0.5] Initialize the Enemy Spawn Point
  (`self.CreateNavPath`)
  (if (`self.UseCachedSpawnTransforms?`)
    (`self.CreateCachedSpawnTransforms`))
  (`self.DisplayWaveSpawnInformation`)
  (return))

(fn `RetrieveCreepSpawnTransform`
  (returns (SpawnTransform :type "Transform Structure"))
  (bind _cachedbotspawntransforms (`self.CachedBotSpawnTransforms`))
  ;[0 1 1 0.5] Used to retrieve a new creep spawn transform for the spawn point
  (if (`self.UseCachedSpawnTransforms?`)
    (return (`KismetArrayLibrary.Array_Get` _cachedbotspawntransforms (`KismetMathLibrary.RandomInteger` (`KismetArrayLibrary.Array_Length` _cachedbotspawntransforms)))) ; Use one of the cached transforms
    (else
      (return (`self.CreateRandomSpawnTransform`)) ; Create a new random transform at runtime
    )))

(fn `SpawnCreep`
  (params (CreepClass :type "/Game/FPSTowerDefenseToolkit/Blueprints/EnemyAI/BP_EnemyAI_Parent Class Reference") (CycleMultiplier :type Integer))
  (locals (Local_CreepSpawnTransform :type "Transform Structure"))
  ;[0 1 1 0.5] Spawns a creep & updates the Creep Actor array
  (set `local.Local_CreepSpawnTransform` (`self.RetrieveCreepSpawnTransform`))
  (bind _returnvalue (`|SpawnActorFromClass` CreepClass (`local.Local_CreepSpawnTransform`) "AlwaysSpawn" "OverrideRootScale" null CycleMultiplier))
  (`/Game/FPSTowerDefenseToolkit/Blueprints/GameplayActors/BP_WaveManager.UpdateCreepActorsArray` (`/Game/FPSTowerDefenseToolkit/Blueprints/FunctionLibraries/BPFL_GetterFunctions.GetWaveManager` self) _returnvalue)
  (return))

(fn `UserConstructionScript`
  (bind _spawningvolume (`self.SpawningVolume`))
  (bind _spawningvolumeradius (`self.SpawningVolumeRadius`))
  (bind (_boxextent_x _boxextent_y _boxextent_z) (`KismetMathLibrary.BreakVector` (`BoxComponent.BoxExtent` _spawningvolume)))
  ;[0 1 1 0.5] Set user defined spline height
  (`SceneComponent.K2_AddLocalOffset` (`self.PathSpline`) (`KismetMathLibrary.MakeVector` 0.0 0.0 (`self.SplineHeight`)) false true)
  (`BoxComponent.SetBoxExtent` _spawningvolume (`KismetMathLibrary.MakeVector` _spawningvolumeradius _spawningvolumeradius _boxextent_z) true))
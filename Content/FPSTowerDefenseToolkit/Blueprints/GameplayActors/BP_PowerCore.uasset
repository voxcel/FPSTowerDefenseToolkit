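; BP_PowerCore is the tower defense objective; when its health reaches zero it explodes and the HUD shows a mission-failed summary.
; Damage updates clamped health, recoloring a dynamic holographic material and the HUD health bar through the player controller.
; Construction precomputes a ring of perimeter points, optionally debug-drawn, handed out randomly so creeps spread out.
; BPI_Targetable functions supply an aim point and radius-corrected distance.
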(event `self.ReceiveAnyDamage`
  (params (Damage :type "Float (single-precision)") (DamageType :type "DamageType Object Reference") (InstigatedBy :type "Controller Object Reference") (DamageCauser :type "Actor Object Reference"))
  ;[1 0.5 0.2 0.5] Reduces health based on damage received; Destroys the core if health goes down to zero; Handle End Game Logic
  (`self.UpdateCoreHealth` (* Damage -1.0))
  (if (not (> (`self.CurrentHealth`) 0.0))
    (`GameplayStatics.SpawnEmitterAtLocation` "/Game/FPSTowerDefenseToolkit/Particles/P_Explosion.P_Explosion" (`SceneComponent.K2_GetComponentLocation` (`self.CollisionSphere`)))
    (bind _asbp_player_hud (cast `/Game/FPSTowerDefenseToolkit/Blueprints/BP_PlayerHUD` (`PlayerController.GetHUD` (`GameplayStatics.GetPlayerController` 0))))
    (`/Game/FPSTowerDefenseToolkit/Blueprints/BP_PlayerHUD.DisplayMissionSummary` _asbp_player_hud false) ; Mission Failed: Request the Player HUD class to Display Mission Summary
    (`self.K2_DestroyActor` self)))

(fn `CreateCoreAttackLocations`
  (locals (Local_AngularDifference :type "Float (double-precision)") (Local_CoreBoundsRadius :type "Float (double-precision)"))
  ;[0 1 1 0.5] Generates a set of locations around the Power Core
  (set `local.Local_CoreBoundsRadius` (+ (`SphereComponent.GetScaledSphereRadius` (`self.CollisionSphere`)) (`self.PerimeterOffset`)))
  (set `local.Local_AngularDifference` (/ 360.0 (`KismetMathLibrary.Conv_IntToDouble` (`self.NumberOfPerimeterPositions`))))
  (for _index (range (`self.NumberOfPerimeterPositions`))
    (bind _returnvalue (* (`KismetMathLibrary.Conv_IntToDouble` _index) (`local.Local_AngularDifference`)))
    (`KismetArrayLibrary.Array_Set` (`self.PerimeterLocationsArray`) _index (`KismetMathLibrary.MakeVector` (+ (.x (`self.K2_GetActorLocation`)) (* (`local.Local_CoreBoundsRadius`) (`KismetMathLibrary.DegCos` _returnvalue))) (+ (.y (`self.K2_GetActorLocation`)) (* (`local.Local_CoreBoundsRadius`) (`KismetMathLibrary.DegSin` _returnvalue))) (.z (`self.K2_GetActorLocation`))) true))
  (return))

(fn `DisplayPerimeterLocations`
  ;[0 1 1 0.5] Displays Core Perimeter locations in the editor
  (for _array_element (`self.PerimeterLocationsArray`)
    (`KismetSystemLibrary.DrawDebugBox` _array_element (20.0 20.0 20.0) (struct :`R` 1.0 :`A` 1.0) (struct) 1.0 3.0))
  (return))

(fn `GetCorrectedDistanceToActor`
  (params (QueringActorLocation :type "Vector Structure"))
  (returns (CorrectedDistance :type "Float (double-precision)"))
  ;[0 1 0.4 0.5] New BPI_Targetable interface function that returns distance from quering actor [Correction required as collision sphere radius is large compared to normal quering actors]
  (return (- (`KismetMathLibrary.VSize` (- QueringActorLocation (`self.K2_GetActorLocation`))) (`SphereComponent.GetScaledSphereRadius` (`self.CollisionSphere`)))))

(fn `InitializePowerCore`
  ;[0 1 1 0.5] Sets the default value of core health in the HUD at the start of the level
  (`self.UpdateCoreHealth` 0.0) ; Zero Increment as HUD updates is the focus & not the health increment itself
  (return))

(fn `RetrieveHealthPercent`
  (returns (ReturnValue :type "Float (double-precision)"))
  (return (/ (`self.CurrentHealth`) (`self.MaxHealth`))))

(fn `RetrieveRandomPerimeterLocation`
  (returns (TargetLocation :type "Vector Structure"))
  (bind _perimeterlocationsarray (`self.PerimeterLocationsArray`))
  ;[0 1 1 0.5] Returns a random perimeter location around the Power Core [Used by creep AI controllers for 'Move To' orders; Random movement target locations prevent all creeps from grouping together in the same area]
  (return (`KismetArrayLibrary.Array_Get` _perimeterlocationsarray (`KismetMathLibrary.RandomInteger` (`KismetArrayLibrary.Array_Length` _perimeterlocationsarray)))))

(fn `RetrieveTargetableLocation`
  (returns (TargetLocation :type "Vector Structure"))
  ;[0 1 0.4 0.5] New BPI_Targetable interface function used by other actors to retrieve the central target location of this actor for launching offensive capabilities
  (return (`SceneComponent.K2_GetComponentLocation` (`self.UnitCore`))))

(fn `SetCoreColor`
  (bind _returnvalue (/ (`self.CurrentHealth`) (`self.MaxHealth`)))
  ;[0 1 1 0.5] Dynamically changes the core's color based on the current health value
  (`MaterialInstanceDynamic.SetVectorParameterValue` (`self.DynamicMatInst_HoloCore`) "GridColor" (`KismetMathLibrary.MakeColor` (- 1.0 _returnvalue) _returnvalue _returnvalue))
  (return))

(fn `UpdateCoreHealth`
  (params (Increment :type "Float (double-precision)"))
  ;[0 1 1 0.5] Updates the Core health, the color of the actor, & the core health progress bar in the HUD
  (set `self.CurrentHealth` (`KismetMathLibrary.FClamp` (+ (`self.CurrentHealth`) Increment) 0.0 (`self.MaxHealth`)))
  (`self.SetCoreColor`)
  (bind _asbp_player_controller (cast `/Game/FPSTowerDefenseToolkit/Blueprints/BP_PlayerController` (`GameplayStatics.GetPlayerController` 0))
    (:`then`
      (`/Game/FPSTowerDefenseToolkit/Blueprints/BP_PlayerController.UpdateHUD_CoreHealthBar` _asbp_player_controller (`self.RetrieveHealthPercent`)) ; Request the Player Controller to update the Core Health bar in the HUD
    )
    (:`CastFailed`
      _))
  (return))

(fn `UserConstructionScript`
  ;[0 1 1 0.5] Set Dynamic Mat Instance for changing core color based on health; Store Core bounds radius for AI Proximity calculations; Set default health
  (bind _returnvalue (`PrimitiveComponent.CreateDynamicMaterialInstance` (`self.CoreMesh`) 0 "/Game/FPSTowerDefenseToolkit/Materials/M_Holographic_Core.M_Holographic_Core"))
  (set `self.DynamicMatInst_HoloCore` _returnvalue)
  (set `self.CurrentHealth` (`self.MaxHealth`))
  (`self.CreateCoreAttackLocations`)
  (if (`self.VisualizePerimeterLocations?`)
    (`self.DisplayPerimeterLocations`)))
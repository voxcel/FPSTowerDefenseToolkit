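; Game state Blueprint for the tower defense toolkit that holds the current gameplay state and the level's mission success flag.
; Initialization sets the default Tower Build Mode through the state update function.
; Each state update stores the new value and has the first player controller, cast to BP_PlayerController, refresh state-based HUD visibility.
; Getter and setter functions expose both values to other Blueprints.
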(fn `InitializeGameState`
  ;[0 1 1 0.5] Initialize the Game State by setting the default state to Tower Build Mode
  (`self.UpdateGameplayState` "NewEnumerator1")
  (return))

(fn `RetrieveGameplayState`
  (returns (GameplayState :type "/Game/FPSTowerDefenseToolkit/Blueprints/Enums/EGameplayState Enum"))
  ;[0 1 1 0.5] Getter function used by other blueprints to retrieve the Gameplay State
  (return (`self.GameplayState`)))

(fn `RetrieveMissionStatus`
  (returns (`MissionSuccess?` :type Boolean))
  ;[0 1 1 0.5] Getter function used by other blueprints to retrieve the mission status
  (return (`self.MissionSuccess?`)))

(fn `UpdateGameplayState`
  (params (NewGameplayState :type "/Game/FPSTowerDefenseToolkit/Blueprints/Enums/EGameplayState Enum"))
  ;[0 1 1 0.5] Updates the Gameplay state; Requests the player controller to make necessary HUD changes for the new state
  (set `self.GameplayState` NewGameplayState)
  (bind _asbp_player_controller (cast `/Game/FPSTowerDefenseToolkit/Blueprints/BP_PlayerController` (`GameplayStatics.GetPlayerController` 0)))
  (`/Game/FPSTowerDefenseToolkit/Blueprints/BP_PlayerController.UpdateHUD_StateBasedVisibility` _asbp_player_controller (`self.GameplayState`)))

(fn `UpdateMissionStatus`
  (params (`Success?` :type Boolean))
  ;[0 1 1 0.5] Update the mission status of the current level
  (set `self.MissionSuccess?` `Success?`)
  (return))

(fn `UserConstructionScript`)
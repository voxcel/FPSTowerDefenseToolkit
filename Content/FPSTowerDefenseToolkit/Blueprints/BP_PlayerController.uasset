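; Player controller for the FPS tower defense game, acting as the gateway between gameplay and the HUD.
; UpdateHUD functions fetch the active HUD widget, cast it to the in-game HUD or tower selection menu, and forward player, ammo, core, tower, target and wave data.
; It also switches between game-only and UI-only input, and possesses and initializes the player character, restoring state-based HUD visibility.
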(fn `EnableInputsForActiveWidgetOnly`
  ;[0 1 1 0.5] Set Input Mode to UI only
  ;;[1 1 1] Version 1.8.1: Replaced deprecated node in v4.13
  (`WidgetBlueprintLibrary.SetInputMode_UIOnlyEx` self (`/Game/FPSTowerDefenseToolkit/Blueprints/FunctionLibraries/BPFL_GetterFunctions.GetActiveHUDWidget`))
  (set `self.bShowMouseCursor` true)
  (return))

(fn `InitializePlayerController`
  ;[0 1 1 0.5] Used to initialize the Player Controller manually instead of relying on the Begin Play Event
  (`WidgetBlueprintLibrary.SetInputMode_GameOnly` self)
  (set `self.bShowMouseCursor` false)
  (return))

(fn `PossessCharacter`
  (params (PlayerCharacter :type "Character Object Reference"))
  ;[0 1 1 0.5] Posses the player character & initialize it
  (`self.Possess` PlayerCharacter)
  (bind _asbp_player_character (cast `/Game/FPSTowerDefenseToolkit/Blueprints/BP_PlayerCharacter` PlayerCharacter))
  (`/Game/FPSTowerDefenseToolkit/Blueprints/BP_PlayerCharacter.InitializePlayerCharacter` _asbp_player_character)
  (`self.UpdateHUD_StateBasedVisibility` (`/Game/FPSTowerDefenseToolkit/Blueprints/FunctionLibraries/BPFL_GetterFunctions.GetGameplayState` self)) ; Takes care of displaying all the necessary UI elements that were hidden during a prior death event
)

(fn `UpdateHUD_AmmoPerMagazine`
  (params (AmmoPerMagazine :type Integer))
  ;[0 1 1 0.5] Request Active HUD Widget to update the Ammo Per Magazine display
  (bind _aswidget_in_game_hud (cast `/Game/FPSTowerDefenseToolkit/UI/Widgets/Widget_InGameHUD` (`/Game/FPSTowerDefenseToolkit/Blueprints/FunctionLibraries/BPFL_GetterFunctions.GetActiveHUDWidget`)))
  (`/Game/FPSTowerDefenseToolkit/UI/Widgets/Widget_InGameHUD.UpdateAmmoPerMagazineText` _aswidget_in_game_hud AmmoPerMagazine))

(fn `UpdateHUD_CoreHealthBar`
  (params (`Health%` :type "Float (double-precision)"))
  ;[0 1 1 0.5] Request Active HUD Widget to update the Core Health Bar
  (bind _aswidget_in_game_hud (cast `/Game/FPSTowerDefenseToolkit/UI/Widgets/Widget_InGameHUD` (`/Game/FPSTowerDefenseToolkit/Blueprints/FunctionLibraries/BPFL_GetterFunctions.GetActiveHUDWidget`)))
  (`/Game/FPSTowerDefenseToolkit/UI/Widgets/Widget_InGameHUD.UpdateCoreHealthBar` _aswidget_in_game_hud `Health%`))

(fn `UpdateHUD_CurrentAmmoCounter`
  (params (AmmoLeft :type Integer))
  ;[0 1 1 0.5] Request Active HUD Widget to update the Current Ammo display
  (bind _aswidget_in_game_hud (cast `/Game/FPSTowerDefenseToolkit/UI/Widgets/Widget_InGameHUD` (`/Game/FPSTowerDefenseToolkit/Blueprints/FunctionLibraries/BPFL_GetterFunctions.GetActiveHUDWidget`)))
  (`/Game/FPSTowerDefenseToolkit/UI/Widgets/Widget_InGameHUD.UpdateCurrentAmmoText` _aswidget_in_game_hud AmmoLeft))

(fn `UpdateHUD_CurrentWaveNumber`
  (params (WaveNumber :type Integer))
  ;[0 1 1 0.5] Request Active HUD Widget to update the current wave number display
  (bind _aswidget_in_game_hud (cast `/Game/FPSTowerDefenseToolkit/UI/Widgets/Widget_InGameHUD` (`/Game/FPSTowerDefenseToolkit/Blueprints/FunctionLibraries/BPFL_GetterFunctions.GetActiveHUDWidget`)))
  (`/Game/FPSTowerDefenseToolkit/UI/Widgets/Widget_InGameHUD.UpdateWaveNumberText` _aswidget_in_game_hud WaveNumber))

(fn `UpdateHUD_DisplayTargetHitPoints`
  (params (TargetName :type Text) (`TargetHealth%` :type "Float (double-precision)"))
  ;[0 1 1 0.5] Request Active HUD Widget to display hitpoints for the target actor
  (bind _aswidget_in_game_hud (cast `/Game/FPSTowerDefenseToolkit/UI/Widgets/Widget_InGameHUD` (`/Game/FPSTowerDefenseToolkit/Blueprints/FunctionLibraries/BPFL_GetterFunctions.GetActiveHUDWidget`)))
  (`/Game/FPSTowerDefenseToolkit/UI/Widgets/Widget_InGameHUD.UpdateTargetHealthBar` _aswidget_in_game_hud TargetName `TargetHealth%`))

(fn `UpdateHUD_DisplayTowerUpgradeStats`
  (params (TowerName :type Text) (CurrentTowerLevel :type Integer) (CurrentDPS :type "Float (double-precision)") (CurrentRange :type "Float (double-precision)") (`CanBeUpgraded?` :type Boolean) (UpgradedTowerLevel :type Integer) (UpgradedDPS :type "Float (double-precision)") (UpgradedRange :type "Float (double-precision)") (UpgradeCost :type Integer))
  ;[0 1 1 0.5] Request Active HUD Widget to display the Tower Upgrade stats
  (bind _aswidget_in_game_hud (cast `/Game/FPSTowerDefenseToolkit/UI/Widgets/Widget_InGameHUD` (`/Game/FPSTowerDefenseToolkit/Blueprints/FunctionLibraries/BPFL_GetterFunctions.GetActiveHUDWidget`)))
  (`/Game/FPSTowerDefenseToolkit/UI/Widgets/Widget_InGameHUD.DisplayTowerUpgradeStats` _aswidget_in_game_hud TowerName CurrentTowerLevel CurrentDPS CurrentRange `CanBeUpgraded?` UpgradedTowerLevel UpgradedDPS UpgradedRange UpgradeCost))

(fn `UpdateHUD_DisplayWaveCountDownTimer`
  (params (CountDownTimerValue :type "Float (double-precision)"))
  ;[0 1 1 0.5] Request Active HUD Widget to display the wave countdown timer UI element
  (bind _aswidget_in_game_hud (cast `/Game/FPSTowerDefenseToolkit/UI/Widgets/Widget_InGameHUD` (`/Game/FPSTowerDefenseToolkit/Blueprints/FunctionLibraries/BPFL_GetterFunctions.GetActiveHUDWidget`)))
  (`/Game/FPSTowerDefenseToolkit/UI/Widgets/Widget_InGameHUD.DisplayWaveCountDownTimer` _aswidget_in_game_hud)
  (`self.UpdateHUD_WaveCountDownTimer` CountDownTimerValue))

(fn `UpdateHUD_HandlePlayerDeathHUDChanges`
  ;[0 1 1 0.5] Request Active HUD Widget to update the visibility of UI elements when the player character is destroyed
  (bind _aswidget_in_game_hud (cast `/Game/FPSTowerDefenseToolkit/UI/Widgets/Widget_InGameHUD` (`/Game/FPSTowerDefenseToolkit/Blueprints/FunctionLibraries/BPFL_GetterFunctions.GetActiveHUDWidget`)))
  (`/Game/FPSTowerDefenseToolkit/UI/Widgets/Widget_InGameHUD.HandlePlayerDeathHUDChanges` _aswidget_in_game_hud))

(fn `UpdateHUD_HideFocusedTargetStatsWidgets`
  ;[0 1 1 0.5] Request Active HUD Widget to hide the focused target stats
  (bind _aswidget_in_game_hud (cast `/Game/FPSTowerDefenseToolkit/UI/Widgets/Widget_InGameHUD` (`/Game/FPSTowerDefenseToolkit/Blueprints/FunctionLibraries/BPFL_GetterFunctions.GetActiveHUDWidget`)))
  (`/Game/FPSTowerDefenseToolkit/UI/Widgets/Widget_InGameHUD.HideFocusedTargetStats` _aswidget_in_game_hud))

(fn `UpdateHUD_HidePlayerStats`
  ;[0 1 1 0.5] Request Active HUD Widget to hide the player stats
  (bind _aswidget_in_game_hud (cast `/Game/FPSTowerDefenseToolkit/UI/Widgets/Widget_InGameHUD` (`/Game/FPSTowerDefenseToolkit/Blueprints/FunctionLibraries/BPFL_GetterFunctions.GetActiveHUDWidget`)))
  (`/Game/FPSTowerDefenseToolkit/UI/Widgets/Widget_InGameHUD.HidePlayerStats` _aswidget_in_game_hud))

(fn `UpdateHUD_HideWaveCountDownTimer`
  ;[0 1 1 0.5] Request Active HUD Widget to hide the wave countdown timer UI element
  (bind _aswidget_in_game_hud (cast `/Game/FPSTowerDefenseToolkit/UI/Widgets/Widget_InGameHUD` (`/Game/FPSTowerDefenseToolkit/Blueprints/FunctionLibraries/BPFL_GetterFunctions.GetActiveHUDWidget`)))
  (`/Game/FPSTowerDefenseToolkit/UI/Widgets/Widget_InGameHUD.HideWaveCountDownTimer` _aswidget_in_game_hud))

(fn `UpdateHUD_InitializePlayerStats`
  (params (`PlayerHealth%` :type "Float (double-precision)") (AmmoLeftInMagazine :type Integer) (MaxAmmoPerMagazine :type Integer))
  ;[0 1 1 0.5] Initialize the player stats HUD elements
  (`self.UpdateHUD_PlayerHealthBar` `PlayerHealth%`)
  (`self.UpdateHUD_CurrentAmmoCounter` AmmoLeftInMagazine)
  (`self.UpdateHUD_AmmoPerMagazine` MaxAmmoPerMagazine)
  (return))

(fn `UpdateHUD_InitializeTowerListBox`
  (params (SelectedTowerIndexArray :type "Array of Integer"))
  ;[0 1 1 0.5] Request Active HUD Widget to populate the Tower List Box
  (bind _aswidget_in_game_hud (cast `/Game/FPSTowerDefenseToolkit/UI/Widgets/Widget_InGameHUD` (`/Game/FPSTowerDefenseToolkit/Blueprints/FunctionLibraries/BPFL_GetterFunctions.GetActiveHUDWidget`)))
  (`/Game/FPSTowerDefenseToolkit/UI/Widgets/Widget_InGameHUD.PopulateTowerListBox` _aswidget_in_game_hud SelectedTowerIndexArray))

(fn `UpdateHUD_InitializeWaveNumberData`
  (params (CurrentWave :type Integer) (`EndlessMode?` :type Boolean) (TotalNumberOfWaves :type Integer))
  ;[0 1 1 0.5] Request Active HUD Widget to initialize the wave number HUD elements
  (bind _aswidget_in_game_hud (cast `/Game/FPSTowerDefenseToolkit/UI/Widgets/Widget_InGameHUD` (`/Game/FPSTowerDefenseToolkit/Blueprints/FunctionLibraries/BPFL_GetterFunctions.GetActiveHUDWidget`)))
  (`/Game/FPSTowerDefenseToolkit/UI/Widgets/Widget_InGameHUD.InitializeWaveNumberData` _aswidget_in_game_hud CurrentWave `EndlessMode?` TotalNumberOfWaves))

(fn `UpdateHUD_NumberOfTowerBases`
  (params (TowerBasesLeft :type Integer))
  ;[0 1 1 0.5] Request Active HUD Widget to update the TowerBases Left display
  (bind _aswidget_in_game_hud (cast `/Game/FPSTowerDefenseToolkit/UI/Widgets/Widget_InGameHUD` (`/Game/FPSTowerDefenseToolkit/Blueprints/FunctionLibraries/BPFL_GetterFunctions.GetActiveHUDWidget`)))
  (`/Game/FPSTowerDefenseToolkit/UI/Widgets/Widget_InGameHUD.UpdateTowerBasesLeftText` _aswidget_in_game_hud TowerBasesLeft))

(fn `UpdateHUD_PlayerHealthBar`
  (params (`CurrentHealth%` :type "Float (double-precision)"))
  ;[0 1 1 0.5] Request Active HUD Widget to update the Player Health Bar
  (bind _aswidget_in_game_hud (cast `/Game/FPSTowerDefenseToolkit/UI/Widgets/Widget_InGameHUD` (`/Game/FPSTowerDefenseToolkit/Blueprints/FunctionLibraries/BPFL_GetterFunctions.GetActiveHUDWidget`)))
  (`/Game/FPSTowerDefenseToolkit/UI/Widgets/Widget_InGameHUD.UpdatePlayerHealthBar` _aswidget_in_game_hud `CurrentHealth%`))

(fn `UpdateHUD_StateBasedVisibility`
  (params (GameplayState :type "/Game/FPSTowerDefenseToolkit/Blueprints/Enums/EGameplayState Enum"))
  ;[0 1 1 0.5] Request Active HUD Widget to handle visibility of UI elements based on the gameplay state
  (bind _aswidget_in_game_hud (cast `/Game/FPSTowerDefenseToolkit/UI/Widgets/Widget_InGameHUD` (`/Game/FPSTowerDefenseToolkit/Blueprints/FunctionLibraries/BPFL_GetterFunctions.GetActiveHUDWidget`)))
  (`/Game/FPSTowerDefenseToolkit/UI/Widgets/Widget_InGameHUD.HandleStateBasedHUDVisibility` _aswidget_in_game_hud GameplayState))

(fn `UpdateHUD_TowerPoints`
  (params (TowerPointsLeft :type Integer))
  ;[0 1 1 0.5] Request Active HUD Widget to update the TowerPoints display
  (bind _aswidget_in_game_hud (cast `/Game/FPSTowerDefenseToolkit/UI/Widgets/Widget_InGameHUD` (`/Game/FPSTowerDefenseToolkit/Blueprints/FunctionLibraries/BPFL_GetterFunctions.GetActiveHUDWidget`)))
  (`/Game/FPSTowerDefenseToolkit/UI/Widgets/Widget_InGameHUD.UpdateTowerPointsLeftText` _aswidget_in_game_hud TowerPointsLeft))

(fn `UpdateHUD_TowerSelectionInformation`
  (params (TowerName :type Text) (TowerDescription :type Text))
  ;[0 1 1 0.5] Request Active HUD Widget to display information about the selected tower
  (bind _aswidget_tower_selection_menu (cast `/Game/FPSTowerDefenseToolkit/UI/Widgets/Widget_TowerSelectionMenu` (`/Game/FPSTowerDefenseToolkit/Blueprints/FunctionLibraries/BPFL_GetterFunctions.GetActiveHUDWidget`)))
  (`/Game/FPSTowerDefenseToolkit/UI/Widgets/Widget_TowerSelectionMenu.UpdateTowerInformationText` _aswidget_tower_selection_menu TowerName TowerDescription))

(fn `UpdateHUD_WaveCountDownTimer`
  (params (CountDownTimer :type "Float (double-precision)"))
  ;[0 1 1 0.5] Request Active HUD Widget to update the wave countdown timer display
  (bind _aswidget_in_game_hud (cast `/Game/FPSTowerDefenseToolkit/UI/Widgets/Widget_InGameHUD` (`/Game/FPSTowerDefenseToolkit/Blueprints/FunctionLibraries/BPFL_GetterFunctions.GetActiveHUDWidget`)))
  (`/Game/FPSTowerDefenseToolkit/UI/Widgets/Widget_InGameHUD.UpdateWaveTimerText` _aswidget_in_game_hud CountDownTimer))

(fn `UserConstructionScript`)
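; Holographic preview of a tower base, following the focused grid cell to show whether placement is allowed.
; Updates from the Tower Spawn Handler check grid tilt, player distance, cell occupancy and bases left, then set placement status and hologram color.
; A gate opened briefly on cell changes limits costly Tower Manager nav path checks.
; Deactivation moves the actor far away so its nav modifier stops affecting the nav mesh.
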(event `self.UpdateDisplayParameters`
  (params (GridCellIndex :type Integer) (GridGeneratorIndex :type Integer) (GridVector :type "Vector Structure") (GridGeneratorRotation :type "Rotator Structure") (GridCellStatus :type "/Game/FPSTowerDefenseToolkit/Blueprints/Enums/EGridCellStatus Enum" :default "NewEnumerator0") (HalfGridSize :type "Float (single-precision)"))
  ;[0 1 1 0.5] Updates display parameters based on input passed in from Tower Spawn Handler; Determines the state of the Holographic Tower
  ;;[1 1 1] Version 1.8.1
  (`self.EvaluateGridDataChanges` GridCellIndex GridGeneratorIndex)
  (`parent.UpdateDisplayParameters` GridCellIndex GridGeneratorIndex GridVector GridGeneratorRotation GridCellStatus HalfGridSize)
  (bind _success_ (`self.ValidateGridRotation`))
  (if _success_
    (bind _actortransform (`self.CreateNewActorTransform` (`self.FocusedGridVector`) (`self.FocusedGridGeneratorRotation`)))
    (set `self.NewActorTransform` _actortransform)
    (bind _success__2 (`self.ValidateDistanceToPlayerCharacter` (`self.FocusedGridVector`) (`self.HalfGridSize`)))
    (if _success__2
      (`self.K2_SetActorTransform` (`self.NewActorTransform`))
      (switch `/Game/FPSTowerDefenseToolkit/Blueprints/Enums/EGridCellStatus` (`self.FocusedGridCellStatus`)
        (:`NewEnumerator0`
          (bind _success__3 (`self.EvaluateTowerResourceRequirements`))
          (if _success__3
            ;;[1 1 1] Version 1.8.1: Improves performance by reducing the number of nav path validation queries
            (if (`self.GridDataChanged?`)
              (`|ExecutionSequence`
                (:`then_0`
                  (goto _label :!via `Open`))
                (:`then_1`
                  (`KismetSystemLibrary.RetriggerableDelay` 0.1)
                  (goto _label :!via `Close`)))
              (else
                (`/Engine/EditorBlueprintResources/StandardMacros.Gate` true :!label _label
                  (:`Exit`
                    (bind _navpathavailable_ (`/Game/FPSTowerDefenseToolkit/Blueprints/GameplayActors/BP_TowerManager.ValidateNavPath` (`/Game/FPSTowerDefenseToolkit/Blueprints/FunctionLibraries/BPFL_GetterFunctions.GetTowerManager` self)))
                    (`self.UpdateTowerPlacementStatus` _navpathavailable_)))))
            (else
              (`self.UpdateTowerPlacementStatus` false :!label _label_2))))
        (:`NewEnumerator1`
          (goto _label_2))
        (:`NewEnumerator2`
          (goto _label_2))
        (:`NewEnumerator3`
          (goto _label_2)))
      (`self.SetHologramColor`)
      (`self.ActivateHoloTower`)
      (else
        (`self.DeactivateHoloTower`)))
    (else
      (`self.DeactivateHoloTower`))))

(event `self.DeactivateHoloTower`
  ;[1 0.5 0.2 0.5] Extend parent function to disable collision for nav modifier volume
  (`parent.DeactivateHoloTower`)
  ;;[1 1 1] Version 1.8.1: Scaling the nav modifier volume down to zero can leave artifacts in the nav mesh under certain conditions; Hence actor instead moved to an isolated location
  (`self.K2_SetActorLocation` (0.0 0.0 50000.0) false true) ; Displace the actor to an isolated location to cancel out the effect of it's nav modifier volume on nav mesh
)

(fn `CreateNewActorTransform`
  (params (GridVector :type "Vector Structure") (GridGeneratorRotation :type "Rotator Structure"))
  (returns (ActorTransform :type "Transform Structure"))
  ;[0 1 1 0.5] Creates new transform based on the focused grid cell & rotation of the focused grid generator
  (return (`KismetMathLibrary.MakeTransform` (`KismetMathLibrary.MakeVector` (.x GridVector) (.y GridVector) (+ (.z GridVector) (`/Game/FPSTowerDefenseToolkit/Blueprints/GameplayActors/BP_TowerManager.TowerBaseZOffset` (`/Game/FPSTowerDefenseToolkit/Blueprints/FunctionLibraries/BPFL_GetterFunctions.GetTowerManager` self)))) (`KismetMathLibrary.MakeRotator` 0.0 0.0 (.yaw GridGeneratorRotation)) (`self.HoloTowerScale`))))

(fn `EvaluateGridDataChanges`
  (params (NewGridCellIndex :type Integer) (NewGridGeneratorIndex :type Integer))
  ;[0 1 1 0.5] Determines if the actor has been moved to a new grid cell
  (set `self.GridDataChanged?` (or (!= NewGridCellIndex (`self.GridCellIndex`)) (!= NewGridGeneratorIndex (`self.GridGeneratorIndex`))))
  (return))

(fn `EvaluateTowerResourceRequirements`
  (returns (`Success?` :type Boolean))
  (bind _asbp_player_state (cast `/Game/FPSTowerDefenseToolkit/Blueprints/BP_PlayerState` (`Controller.PlayerState` (`GameplayStatics.GetPlayerController` 0)))
    (:`then`
      (return (> (`/Game/FPSTowerDefenseToolkit/Blueprints/BP_PlayerState.RetrieveTowerBasesLeft` _asbp_player_state) 0)))
    (:`CastFailed`
      (return false))))

(fn `UserConstructionScript`
  (`parent.UserConstructionScript`))

(fn `ValidateDistanceToPlayerCharacter`
  (params (GridVector :type "Vector Structure") (MinRequiredDistance :type "Float (double-precision)"))
  (returns (`Success?` :type Boolean))
  ;[0 1 1 0.5] Makes sure that towers do not spawn if player is blocking the spawn position
  (return (> (`KismetMathLibrary.VSize` (- GridVector (`self.K2_GetActorLocation` (`GameplayStatics.GetPlayerCharacter` 0)))) MinRequiredDistance)))

(fn `ValidateGridRotation`
  (returns (`Success?` :type Boolean))
  (bind (_focusedgridgeneratorrotation_roll _focusedgridgeneratorrotation_pitch) (`KismetMathLibrary.BreakRotator` (`self.FocusedGridGeneratorRotation`)))
  (bind _maxgridgeneratorinclination (`self.MaxGridGeneratorInclination`))
  ;[0 1 1 0.5] Restricts the tower base placements to grid generators with inclination less than the max supported value
  (return (and (< _focusedgridgeneratorrotation_roll _maxgridgeneratorinclination) (< _focusedgridgeneratorrotation_pitch _maxgridgeneratorinclination))))
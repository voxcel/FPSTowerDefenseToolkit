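; Parent Blueprint for enemy creep bots that advance on the Power Core in the tower defense game.
; Construction scales health by the square root of bot level, and BeginPlay moves the bot to a random point on the core's perimeter.
; Damage feeds a clamped health update, with death reported to BP_GameMode for destruction and an explosion spawned on EndPlay.
; Interface functions serve targeting and HUD health display, while attack animation hooks await child classes.
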(event `self.ReceiveBeginPlay`
  ;[0 1 1 0.5] Gets a perimeter location around the Core & move towards it
  (set `self.CoreTargetLocation` (`/Game/FPSTowerDefenseToolkit/Blueprints/GameplayActors/BP_PowerCore.RetrieveRandomPerimeterLocation` (`/Game/FPSTowerDefenseToolkit/Blueprints/FunctionLibraries/BPFL_GetterFunctions.GetPowerCore` self)))
  (`self.MoveToCore`))

(event `self.ReceiveAnyDamage`
  (params (Damage :type "Float (single-precision)") (DamageType :type "DamageType Object Reference") (InstigatedBy :type "Controller Object Reference") (DamageCauser :type "Actor Object Reference"))
  ;[1 0 0 0.5] Receive Damage; Destroy self if health becomes less than or equal to zero; Activate Termination Protocols
  (`self.UpdateHealth` (* Damage -1.0))
  (if (not (> (`self.UnitHealth`) 0.0))
    (`self.ActivateTerminationProtocols`)))

(event `self.ReceiveEndPlay`
  (params (EndPlayReason :type "EEndPlayReason Enum" :default "Destroyed"))
  ;[1 0 0 0.5] Spawn Explosion Particle when destroyed
  (`GameplayStatics.SpawnEmitterAtLocation` "/Game/FPSTowerDefenseToolkit/Particles/P_Explosion.P_Explosion" (`self.K2_GetActorLocation`)))

(event `/Game/FPSTowerDefenseToolkit/Blueprints/Interfaces/BPI_HUDStatsUpdates.DisplayHUDStats`
  ;[0 1 0.4 0.5] 'BPI_HUDStatsUpdates' interface function used to display the hit points stats of the targeted creep
  (bind _asbp_player_controller (cast `/Game/FPSTowerDefenseToolkit/Blueprints/BP_PlayerController` (`GameplayStatics.GetPlayerController` 0)))
  (`/Game/FPSTowerDefenseToolkit/Blueprints/BP_PlayerController.UpdateHUD_DisplayTargetHitPoints` _asbp_player_controller (`KismetTextLibrary.Conv_StringToText` (`|GetEnumeratorNameAsString` (`self.BotType`))) (/ (`self.UnitHealth`) (`self.MaxHealth`))))

(fn `ActivateTerminationProtocols`
  ;[1 0 0 0.5] Report pending destruction to Game Mode; Game Mode handles the rest
  (`/Game/FPSTowerDefenseToolkit/Blueprints/BP_GameMode.ReportCreepPendingDestroy` (cast `/Game/FPSTowerDefenseToolkit/Blueprints/BP_GameMode` (`GameplayStatics.GetGameMode`) :!pure true) self))

(fn `EndPlaceholderAttackAnimation`
  ;[0 1 1 0.5] Implemented through child classes
)

(fn `FocusViewOnTarget`
  (params (Target :type "Actor Object Reference"))
  ;[0 1 1 0.5] Turn to face the target
  (`/Engine/EditorBlueprintResources/StandardMacros.IsValid` Target
    (:`Is Valid`
      (`self.K2_SetActorRotation` (`KismetMathLibrary.MakeRotator` (.roll (`self.K2_GetActorRotation`)) (.pitch (`self.K2_GetActorRotation`)) (.yaw (`KismetMathLibrary.FindLookAtRotation` (`self.K2_GetActorLocation`) (`self.K2_GetActorLocation` Target))))))
    (:`Is Not Valid`
      _))
  (return))

(fn `GetCorrectedDistanceToActor`
  (params (QueringActorLocation :type "Vector Structure"))
  (returns (CorrectedDistance :type "Float (double-precision)"))
  ;[0 1 0.4 0.5] BPI_Targetable interface function that returns distance from quering actor [No correction required as capsule radius is small]
  (return (`KismetMathLibrary.VSize` (- QueringActorLocation (`self.K2_GetActorLocation`)))))

(fn `MoveToCore`
  ;[0 1 1 0.5] Move towards the Core
  (bind _returnvalue (`AIBlueprintHelperLibrary.GetAIController` self))
  (`AIController.MoveToLocation` _returnvalue (`self.CoreTargetLocation`) 0.0 false true false false null true))

(fn `RetrieveTargetableLocation`
  (returns (TargetLocation :type "Vector Structure"))
  ;[0 1 0.4 0.5] BPI_Targetable interface function used by other actors to retrieve the central target location of this actor for launching offensive capabilities
  (return (`SceneComponent.K2_GetComponentLocation` (`self.UnitCore`))))

(fn `StartPlaceholderAttackAnimation`
  ;[0 1 1 0.5] Implemented through child classes
)

(fn `UpdateHealth`
  (params (Increment :type "Float (double-precision)"))
  ;[0 1 1 0.5] New function to handle health updates; Enables both internal & external health update requests to pass through the same conduit
  (set `self.UnitHealth` (`KismetMathLibrary.FClamp` (+ (`self.UnitHealth`) Increment) 0.0 (`self.MaxHealth`)))
  (return))

(fn `UserConstructionScript`
  ;[0 1 1 0.5] Increases Unit Resilience to increase the difficulty with each wave cycle.
  (bind _output_get (set `self.MaxHealth` (* (`self.MaxHealth`) (`KismetMathLibrary.Sqrt` (`KismetMathLibrary.Conv_IntToDouble` (`self.BotLevel`))))))
  (set `self.UnitHealth` _output_get))